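; BP_Gate is a gate actor whose only live behavior is playing a sound at its Box trigger's location on any overlap.
; An unconnected chain holds a streamed level transition: show a widget, disable input, load LevelToLoad, move an actor to Capsule, restore input and unload CurrentLevel.
; An older open-level call with DestinationTag options is also left unconnected, so the gate changes no levels.
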(event `self.Box.OnComponentBeginOverlap`
  (params (OverlappedComponent :type "PrimitiveComponent Object Reference") (OtherActor :type "Actor Object Reference") (OtherComp :type "PrimitiveComponent Object Reference") (OtherBodyIndex :type Integer) (bFromSweep :type Boolean) (SweepResult :type "HitResult Structure (by ref)"))
  (`GameplayStatics.PlaySoundAtLocation` null (`SceneComponent.K2_GetComponentLocation` (`self.Box`)) (struct) 1.0 1.0 0.0 null null null null))

(fn `UserConstructionScript`)