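; Inventory component that stores picked-up items in 12 slots and displays them through a W_HeldItembox widget.
; On Interact, a sphere trace at player 0's location looks for a BP_TestIngredient.
; A slot loop stacks it onto a matching stackable item or fills an empty slot, whichever comes first, then refreshes the widget and destroys the actor.
; Tick re-adds the widget to the viewport whenever it is not visible.
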(event `self.ReceiveBeginPlay`
  ;[0.6291 0.2185 1] Inventory Structure
  (bind _returnvalue (`|CreateWidget` "/Game/UI/W_HeldItembox.W_HeldItembox_C"))
  (set `self.InventoryWidget` _returnvalue)
  (`KismetArrayLibrary.Array_Resize` (`self.Items`) 12)
  (`/Game/UI/W_HeldItembox.LoadItem` (`self.InventoryWidget`) self))

(event `EnhancedInput|/Game/ThirdPerson/Input/Actions/IA_Interact`
  (params (ActionValue :type Boolean) (ElapsedSeconds :type "Float (double-precision)") (TriggeredSeconds :type "Float (double-precision)") (InputAction :type "InputAction Object Reference" :default "/Game/ThirdPerson/Input/Actions/IA_Interact.IA_Interact"))
  (bind _returnvalue (- (`Actor.K2_GetActorLocation` (`GameplayStatics.GetPlayerCharacter` 0)) (0.0 0.0 0.0)))
  ;[0.1168 1 0.08209] Item Detection
  (:`Triggered`
    (bind _outhit (`KismetSystemLibrary.SphereTraceSingle` _returnvalue _returnvalue 50.0 "TraceTypeQuery1"))
    (bind _asbp_test_ingredient (cast `/Game/Inventory/Ingredients/BP_TestIngredient` (`.HitActor` (`GameplayStatics.BreakHitResult` _outhit))))
    ;[0 0.9326 1] Pickup Item Info + Inventory Update
    (for (_array_element _array_index) (`self.Items`)
      (`/Engine/EditorBlueprintResources/StandardMacros.IsValid` _asbp_test_ingredient
        (:`Is Valid`
          (bind (_name _thumbnail _itemclass _quantity) (break `/Game/Inventory/FItemStruct` _array_element))
          (bind (_name_2 _thumbnail_2 _itemclass_2 _quantity_2 _stackable) (break `/Game/Inventory/FItemStruct` (`/Game/Inventory/Ingredients/BP_TestIngredient.Item` _asbp_test_ingredient)))
          (if (and (== _name _name_2) _stackable)
            (bind (_item_name _item_thumbnail _item_itemclass _item_quantity _item_stackable) (break `/Game/Inventory/FItemStruct` (`/Game/Inventory/Ingredients/BP_TestIngredient.Item` _asbp_test_ingredient)))
            (`KismetArrayLibrary.Array_Set` (`self.Items`) _array_index (make `/Game/Inventory/FItemStruct` _item_name _item_thumbnail _item_itemclass (+ _quantity _quantity_2) _item_stackable))
            (`/Game/UI/W_HeldItembox.LoadItem` (`self.InventoryWidget`) self :!label _label)
            (`Actor.K2_DestroyActor` _asbp_test_ingredient)
            (elif (== _quantity 0)
              (`KismetArrayLibrary.Array_Set` (`self.Items`) _array_index (`/Game/Inventory/Ingredients/BP_TestIngredient.Item` _asbp_test_ingredient))
              (goto _label))))))))

(event `self.ReceiveTick`
  (params (DeltaSeconds :type "Float (single-precision)"))
  ;[1 0.8845 0.1996] Display Inventory UI
  (if (not (`Widget.IsVisible` (`self.InventoryWidget`)))
    (`UserWidget.AddToViewport` (`self.InventoryWidget`) 0)))